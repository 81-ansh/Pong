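; BP_Paddle is a player-controlled paddle that slides along its local X axis.
; BeginPlay registers the IMC_Paddle Enhanced Input mapping context with the first player controller.
; While IA_Move triggers, it stores the input as MovementDirection and applies a swept local offset scaled by Speed, without delta-time scaling.
; MovementDirection resets to zero only when the action is canceled.
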(event `self.ReceiveBeginPlay`
  ;[1 1 0 0.5] Add Mapping Context
  (`EnhancedInputSubsystemInterface.AddMappingContext` (pcsubsystem `EnhancedInputLocalPlayerSubsystem` (`GameplayStatics.GetPlayerController` 0)) "/Game/Input/IMC_Paddle.IMC_Paddle" 0 (struct)))

(event `EnhancedInput|/Game/Input/IA_Move`
  (params (ActionValue :type "Float (double-precision)") (ElapsedSeconds :type "Float (double-precision)") (TriggeredSeconds :type "Float (double-precision)") (InputAction :type "InputAction Object Reference" :default "/Game/Input/IA_Move.IA_Move"))
  ;[0 1 0 0.5] Handle Movement
  (:`Triggered`
    (set `self.MovementDirection` ActionValue)
    (`self.K2_AddActorLocalOffset` (`KismetMathLibrary.MakeVector` (* (`self.MovementDirection`) (`self.Speed`))) true))
  (:`Canceled`
    (set `self.MovementDirection` 0.0)))

(fn `UserConstructionScript`)